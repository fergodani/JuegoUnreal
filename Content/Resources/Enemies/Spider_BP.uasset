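; Spider enemy that chases the player, attacks at close range and can be killed.
; A looping timer re-issues AI MoveTo toward the player, while Tick checks distance and triggers AtacarJugador when in range.
; A DoOnce gate paces attacks, raising IsAttack during a delay, then damaging the first-person character without rechecking range.
; ReducirVida subtracts Life per call, and at zero decrements the game mode's enemy count and destroys the spider.
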(event `self.ReceiveBeginPlay`
  (`KismetSystemLibrary.K2_SetTimer` null "SeguirJugador" 1.0 true)
  (set `self.life` 40))

(event `self.ReceiveActorBeginOverlap`
  (params (OtherActor :type "Actor Object Reference")))

(event `self.ReceiveTick`
  (params (DeltaSeconds :type "Float (single-precision)"))
  (if (<= (`self.GetDistanceTo` (`GameplayStatics.GetPlayerPawn` 0) self) 200.0)
    (`self.AtacarJugador`)))

(event `SeguirJugador`
  (`|AIMoveTo` self (0.0 0.0 0.0) (`GameplayStatics.GetPlayerCharacter` 0) 100.0))

(event `ReducirVida`
  (`KismetSystemLibrary.PrintString` "reducri vida")
  (bind _output_get (set `self.life` (- (`self.life`) 20)))
  (if (<= _output_get 0)
    (bind _asfirst_person_game_mode (cast `/Game/FirstPersonBP/Blueprints/FirstPersonGameMode` (`GameplayStatics.GetGameMode`)))
    (`/Game/FirstPersonBP/Blueprints/FirstPersonGameMode.DecrementEnemies` _asfirst_person_game_mode)
    (`self.K2_DestroyActor`)))

(event `AtacarJugador`
  (`/Engine/EditorBlueprintResources/StandardMacros.DoOnce` false :!label _label
    (:`Completed`
      (set `self.isAttack` true)
      (`KismetSystemLibrary.Delay` 1.0)
      (set `self.isAttack` false)
      (bind _asfirst_person_character (cast `/Game/FirstPersonBP/Blueprints/FirstPersonCharacter` (`GameplayStatics.GetPlayerPawn` 0)))
      (`/Game/FirstPersonBP/Blueprints/FirstPersonCharacter.Impactado` _asfirst_person_character 20)
      (goto _label :!via `Reset`))))

(fn `UserConstructionScript`)