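; CraftingTable_BP is a crafting table actor that opens the crafting menu when the player walks into it.
; On overlap with a FirstPersonCharacter, it creates the CraftingMenu widget only if no valid one is cached, then adds it to the viewport.
; It also shows the mouse cursor, switches input to UI only with focus on the menu, and pauses the game.
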(event `self.ReceiveActorBeginOverlap`
  (params (OtherActor :type "Actor Object Reference"))
  (bind _returnvalue (`GameplayStatics.GetPlayerController` 0))
  (bind _craftingmenu (`self.CraftingMenu`))
  (cast `/Game/FirstPersonBP/Blueprints/FirstPersonCharacter` OtherActor)
  (`/Engine/EditorBlueprintResources/StandardMacros.IsValid` (`self.CraftingMenu`)
    (:`Is Valid`
      _)
    (:`Is Not Valid`
      (bind _returnvalue_2 (`|CreateWidget` "/Game/FirstPersonBP/Blueprints/CraftingMenu.CraftingMenu_C"))
      (set `self.CraftingMenu` _returnvalue_2)))
  (set `PlayerController.bShowMouseCursor` true _returnvalue)
  (`WidgetBlueprintLibrary.SetInputMode_UIOnlyEx` _returnvalue _craftingmenu)
  (`UserWidget.AddToViewport` _craftingmenu 0)
  (`GameplayStatics.SetGamePaused` true))

(fn `UserConstructionScript`)