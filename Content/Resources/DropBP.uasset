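; DropBP is a resource pickup that transfers its stored coal, iron, amethyst, torches and ammo to the FirstPersonCharacter that overlaps it.
; On actor overlap it casts to the character and adds the three minerals through their Increment functions.
; Torch and ammo counts are assigned directly, replacing the character's current values instead of adding to them.
; The drop then destroys itself, while other overlapping actors are ignored.
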(event `self.ReceiveActorBeginOverlap`
  (params (OtherActor :type "Actor Object Reference"))
  (bind _asfirst_person_character (cast `/Game/FirstPersonBP/Blueprints/FirstPersonCharacter` OtherActor))
  (`/Game/FirstPersonBP/Blueprints/FirstPersonCharacter.IncrementCoal` _asfirst_person_character (`self.storedCoal`))
  (`/Game/FirstPersonBP/Blueprints/FirstPersonCharacter.IncrementIron` _asfirst_person_character (`self.storedIron`))
  (`/Game/FirstPersonBP/Blueprints/FirstPersonCharacter.IncrementAmethyst` _asfirst_person_character (`self.storedAmethyst`))
  (set `/Game/FirstPersonBP/Blueprints/FirstPersonCharacter.Torchs` (`self.storedTorchs`) _asfirst_person_character)
  (set `/Game/FirstPersonBP/Blueprints/FirstPersonCharacter.Ammo` (`self.storedAmmo`) _asfirst_person_character)
  (`self.K2_DestroyActor`))

(fn `UserConstructionScript`)