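; BP_Lich is an enemy lich character that chases the player and casts spells at them.
; A looping timer moves it toward the player, and Tick triggers a do-once attack within range that halts movement, then spawns an EnemieSpell_BP aimed at the player's mesh with a sound.
; ReducirVida briefly stuns it and subtracts life, and at zero it decrements the FirstPersonGameMode lich count and destroys itself.
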(event `self.ReceiveBeginPlay`
  (`KismetSystemLibrary.K2_SetTimer` null "SeguirJugador" 1.0 true)
  (set `self.life` 100))

(event `self.ReceiveTick`
  (params (DeltaSeconds :type "Float (single-precision)"))
  (`KismetSystemLibrary.Delay` 1.5)
  (if (<= (`self.GetDistanceTo` (`GameplayStatics.GetPlayerPawn` 0) self) 3000.0)
    (`self.AtacarJugador`)))

(event `SeguirJugador`
  (`|AIMoveTo` self (0.0 0.0 0.0) (`GameplayStatics.GetPlayerCharacter` 0) 100.0))

(event `AtacarJugador`
  (bind _returnvalue (`SceneComponent.K2_GetComponentLocation` (`self.SpellSpawnLocation`)))
  (`/Engine/EditorBlueprintResources/StandardMacros.DoOnce` false :!label _label
    (:`Completed`
      (set `self.isAttack` true)
      (`CharacterMovementComponent.DisableMovement` (`self.CharacterMovement`))
      (`KismetSystemLibrary.Delay` 1.2)
      (`|SpawnActorFromClass` "/Game/UndeadPack/Lich/Blueprint/EnemieSpell_BP.EnemieSpell_BP_C" (`KismetMathLibrary.MakeTransform` _returnvalue (`KismetMathLibrary.FindLookAtRotation` _returnvalue (`SceneComponent.K2_GetComponentLocation` (`Character.Mesh` (`GameplayStatics.GetPlayerCharacter` 0))))) "Undefined" "OverrideRootScale" null null)
      (`GameplayStatics.PlaySoundAtLocation` "/Game/UndeadPack/Lich/Blueprint/SpellSound.SpellSound" (`self.K2_GetActorLocation`) (struct) 1.0 1.0 0.0 null null null)
      (set `self.isAttack` false)
      (`CharacterMovementComponent.SetMovementMode` (`self.CharacterMovement`) "MOVE_Walking" 0)
      (goto _label :!via `Reset`))))

(event `ReducirVida`
  (set `self.isImpacted` true)
  (`CharacterMovementComponent.DisableMovement` (`self.CharacterMovement`))
  (`KismetSystemLibrary.Delay` 1.0)
  (set `self.isImpacted` false)
  (`CharacterMovementComponent.SetMovementMode` (`self.CharacterMovement`) "MOVE_Walking" 0)
  (`KismetSystemLibrary.PrintString` "reducri vida")
  (bind _output_get (set `self.life` (- (`self.life`) 20)))
  (if (<= _output_get 0)
    (`CharacterMovementComponent.DisableMovement` (`self.CharacterMovement`))
    (bind _asfirst_person_game_mode (cast `/Game/FirstPersonBP/Blueprints/FirstPersonGameMode` (`GameplayStatics.GetGameMode`)))
    (`/Game/FirstPersonBP/Blueprints/FirstPersonGameMode.DecrementLich` _asfirst_person_game_mode)
    (set `self.isDead` true)
    (`KismetSystemLibrary.Delay` 1.0)
    (set `self.isDead` false)
    (`self.K2_DestroyActor`)))

(fn `UserConstructionScript`)