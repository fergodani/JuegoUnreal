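; Chest actor that stores coal, iron and amethyst, and brings up a final menu once enough amethyst is deposited.
; Overlap by the first-person character registers the chest on that character, opens a reusable chest widget with UI-only input and pauses the game.
; Custom events increment or decrement each stored count without bounds checks.
; Reaching the amethyst threshold swaps the chest widget for the final menu and unpauses.
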(event `self.ReceiveActorBeginOverlap`
  (params (OtherActor :type "Actor Object Reference"))
  (bind _returnvalue (`GameplayStatics.GetPlayerController` 0))
  (bind _chestmenu (`self.ChestMenu`))
  (bind _asfirst_person_character (cast `/Game/FirstPersonBP/Blueprints/FirstPersonCharacter` OtherActor))
  (set `/Game/FirstPersonBP/Blueprints/FirstPersonCharacter.Chest` self _asfirst_person_character)
  (`/Engine/EditorBlueprintResources/StandardMacros.IsValid` (`self.ChestMenu`)
    (:`Is Valid`
      _)
    (:`Is Not Valid`
      (bind _returnvalue_2 (`|CreateWidget` "/Game/FirstPersonBP/Blueprints/ChestMenu.ChestMenu_C"))
      (set `self.ChestMenu` _returnvalue_2)))
  (set `PlayerController.bShowMouseCursor` true _returnvalue)
  (`WidgetBlueprintLibrary.SetInputMode_UIOnlyEx` _returnvalue _chestmenu)
  (`UserWidget.AddToViewport` _chestmenu 0)
  (`GameplayStatics.SetGamePaused` true))

(event `StoreCoal`
  ;[1 1 1] Store Items
  (set `self.StoredCoal` (+ (`self.StoredCoal`) 1)))

(event `RetrieveCoal`
  ;[1 1 1] Retrieve Itmems
  (set `self.StoredCoal` (- (`self.StoredCoal`) 1)))

(event `RetrieveIron`
  ;[1 1 1] Retrieve Itmems
  (set `self.StoredIron` (- (`self.StoredIron`) 1)))

(event `StoreIron`
  ;[1 1 1] Store Items
  (set `self.StoredIron` (+ (`self.StoredIron`) 1)))

(event `RetrieveAmethyst`
  ;[1 1 1] Retrieve Itmems
  (set `self.StoredAmethyst` (- (`self.StoredAmethyst`) 1)))

(event `StoreAmethyst`
  ;[1 1 1] Store Items
  (set `self.StoredAmethyst` (+ (`self.StoredAmethyst`) 1))
  (if (>= (`self.StoredAmethyst`) 25)
    (bind _returnvalue (`|CreateWidget` "/Game/FirstPersonBP/Blueprints/FinalMenu.FinalMenu_C"))
    (bind _output_get (set `self.FinalMenu` _returnvalue))
    (`WidgetBlueprintLibrary.SetInputMode_UIOnlyEx` (`GameplayStatics.GetPlayerController` 0) _output_get)
    (`UserWidget.AddToViewport` _output_get 0)
    (`Widget.RemoveFromParent` (`self.ChestMenu`))
    (`GameplayStatics.SetGamePaused` false)))

(fn `UserConstructionScript`)